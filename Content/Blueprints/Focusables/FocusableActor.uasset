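; FocusableActor is an actor the player can focus on, with a floating nameplate and a focus highlight.
; On BeginPlay it writes FocusNameplate into its nameplate widget and caches the player character.
; Every tick it rotates the nameplate to face the player's camera.
; Focus and ReleiveFocus toggle the indicator decal and custom depth rendering on the first primitive component tagged "outline".
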(event EventBeginPlay
  (bind _asnameplate_widget (Utilities|Casting|CastToNameplateWidget (UserInterface|GetUserWidgetObject (Variables|Default|GetnameplateWidgetComponent))))
  (Variables|/Game/Blueprints/NameplateWidget.NameplateWidget_C|SetunitNameString _asnameplate_widget (Utilities|String|ToString(Name) (Variables|HUDinfo|GetfocusNameplate)))
  (bind _mycharacter (CallFunction|GetPlayerCharacterasMyCharacter))
  (Variables|Default|SetplayerCharacter _mycharacter))

(event Collision|EventActorBeginOverlap
  (params (OtherActor :type Actor%20Object%20Reference)))

(event EventFocus
  (Rendering|SetRenderCustomDepth (Utilities|Array|Get(acopy) (Actor|GetComponentsbyTag "/Script/Engine.PrimitiveComponent" "outline")) true)
  (Rendering|SetVisibility (Variables|Default|GetfocusIndicatorDecal) true false))

(event EventReleiveFocus
  (Rendering|SetRenderCustomDepth (Utilities|Array|Get(acopy) (Actor|GetComponentsbyTag "/Script/Engine.PrimitiveComponent" "outline")) false)
  (Rendering|SetVisibility (Variables|Default|GetfocusIndicatorDecal) false false))

(event EventTick
  (params (DeltaSeconds :type Float%20%28single-precision%29))
  (bind _nameplatewidgetcomponent (Variables|Default|GetnameplateWidgetComponent))
  (Transformation|SetWorldRotation _nameplatewidgetcomponent (Math|Rotator|FindLookatRotation (Transformation|GetWorldLocation _nameplatewidgetcomponent) (Transformation|GetWorldLocation (Variables|/Game/Blueprints/MyCharacter.MyCharacter_C|GetCamera (Variables|Default|GetplayerCharacter)))) false false))

(fn ConstructionScript)