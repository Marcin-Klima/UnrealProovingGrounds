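; Player controller Blueprint that routes movement, turning and jump input to the player's character.
; On BeginPlay it caches player character 0, then forward and strafe axes add movement along vectors from that character's control rotation.
; A look axis drives controller yaw only, with no pitch input, and pressing Jump triggers the character's jump.
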(event EventBeginPlay
  (Variables|Default|SetMyCharacter (Game|GetPlayerCharacter 0)))

(event EventTick
  (params (DeltaSeconds :type Float%20%28single-precision%29)))

(event Input|ActionEvents|InputActionJump
  (params (Key :type Key%20Structure :default "None"))
  ;[1 1 1] View
  (:Pressed
    (Character|Jump (Variables|Default|GetMyCharacter))))

(event Input|AxisEvents|InputAxisLookLeftRight
  (params (AxisValue :type Float%20%28single-precision%29))
  ;[1 1 1] View
  (Pawn|Input|AddControllerYawInput (Variables|Default|GetMyCharacter) AxisValue))

(event Input|AxisEvents|InputAxisMoveForwardBackward
  (params (AxisValue :type Float%20%28single-precision%29))
  (bind _mycharacter (Variables|Default|GetMyCharacter))
  ;[1 1 1] Moving Functionality
  (Pawn|Input|AddMovementInput _mycharacter (Math|Vector|GetForwardVector (Pawn|GetControlRotation _mycharacter :!class /Script/Engine.Pawn)) AxisValue false))

(event Input|AxisEvents|InputAxisMoveLeftRight
  (params (AxisValue :type Float%20%28single-precision%29))
  (bind _mycharacter (Variables|Default|GetMyCharacter))
  ;[1 1 1] Moving Functionality
  (Pawn|Input|AddMovementInput _mycharacter (Math|Vector|GetRightVector (Pawn|GetControlRotation _mycharacter :!class /Script/Engine.Pawn)) AxisValue false))

(fn ConstructionScript)