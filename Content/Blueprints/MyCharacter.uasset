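; MyCharacter is a character Blueprint that tracks one focused FocusableActor, set from a hit actor that a comment describes as clicked.
; SetFocusActor casts the hit, releases any previous focus and selects a different target, or clears focus when the hit is invalid.
; Select and Unselect helpers store or clear FocusedActor and notify it.
; The event graph is inactive, holding only empty events and an unconnected sphere-overlap query.
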(event EventBeginPlay)

(event Collision|EventActorBeginOverlap
  (params (OtherActor :type Actor%20Object%20Reference)))

(event EventTick
  (params (DeltaSeconds :type Float%20%28single-precision%29)))

(fn ConstructionScript)

(fn SetFocusActor
  (params (isObjectValid :type Boolean) (hitActor :type Actor%20Object%20Reference))
  ;[1 1 1] Check if user clicked on fucusable actor
  (if isObjectValid
    (bind _asfocusable_actor (Utilities|Casting|CastToFocusableActor hitActor))
    (if (not (== _asfocusable_actor (Variables|Default|GetfocusedActor)))
      (Utilities|IsValid (Variables|Default|GetfocusedActor)
        (:Is%20Valid
          (CallFunction|UnselectFocusActor))
        (:Is%20Not%20Valid
          _))
      (CallFunction|SelectFocusActor _asfocusable_actor))
    (else
      (Utilities|IsValid (Variables|Default|GetfocusedActor)
        (:Is%20Valid
          (CallFunction|UnselectFocusActor))))))

(fn UnselectFocusActor
  (Default|ReleiveFocus (Variables|Default|GetfocusedActor))
  (Variables|Default|SetfocusedActor 0))

(fn SelectFocusActor
  (params (focusableActor :type Focusable%20Actor%20Object%20Reference))
  (bind _output_get (Variables|Default|SetfocusedActor focusableActor))
  (Default|ReceiveFocus _output_get))